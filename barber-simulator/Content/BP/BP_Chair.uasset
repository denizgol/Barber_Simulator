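; Interactable chair that seats the interacting character and offers the player a timed E tap-key prompt on trigger overlap.
; StartInteraction disables movement, plays a sitting montage, moves the character onto the seat, starts an NPC key timer and passes the chair location to the player character.
; EndInteraction calls ReleaseChair, which moves the character to StandLocation and restores movement.
; CostumerCome? is empty, leaving its TapKey collision toggle disconnected.
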(event OnComponentBeginOverlap(Tap_key)
  (params (OverlappedComponent :type Primitive%20Component%20Object%20Reference) (OtherActor :type Actor%20Object%20Reference) (OtherComp :type Primitive%20Component%20Object%20Reference) (OtherBodyIndex :type Integer) (bFromSweep :type Boolean) (SweepResult :type Hit%20Result%20Structure%20%28by%20ref%29))
  (bind _returnvalue (Game|GetPlayerController 0))
  (bind _returnvalue_2 (Pawn|GetControlledPawn _returnvalue))
  ;[1 1 1] Create Tap Key Event
  (if (== OtherActor _returnvalue_2)
    (bind _asbp_third_person_character (Utilities|Casting|CastToBP_ThirdPersonCharacter _returnvalue_2))
    (Default|CreateTapKeyEvent _asbp_third_person_character "E" "E" true (Math|Random|RandomFloatinRange 0.2 0.3) self)))

(event Custom|ReleaseChair
  (bind _character (Variables|Default|GetCharacter))
  ;[1 1 1] Release Chair
  (bind _character_2 (Variables|Default|GetCharacter)
    (:then
      (Animation|StopAnimMontage _character_2 "/Game/Characters/Mannequins/Animations/Manny/AI_Actions/Male_Sitting_Pose_Montage.Male_Sitting_Pose_Montage")
      (Components|MoveComponentTo (Variables|/Script/Engine.Actor|GetRootComponent _character) (+ (Math|Vector|MakeVector 0.0 0.0 (Variables|/Script/Engine.CapsuleComponent|GetCapsuleHalfHeight (Variables|/Script/Engine.Character|GetCapsuleComponent _character))) (Transformation|GetWorldLocation (Variables|Default|GetStandLocation))) (Transformation|GetActorRotation _character) false false 0.5 false)
      (Class|BPICharacter|ToggleMovement(Message) (Variables|Default|GetCharacter) true))
    (:else)))

(event EventBeginPlay
  ;[1 1 1] start
  (|CallParentFunction))

(event Collision|EventActorBeginOverlap
  (params (OtherActor :type Actor%20Object%20Reference))
  ;[1 1 1] start
  (|CallParentFunction OtherActor) ; This node is disabled and will not be called.\nDrag off pins to build functionality.
)

(event EventTick
  (params (DeltaSeconds :type Float%20%28single-precision%29))
  ;[1 1 1] start
  (|CallParentFunction DeltaSeconds) ; This node is disabled and will not be called.\nDrag off pins to build functionality.
)

(event EventStartInteraction
  (params (InteractingCharacter :type Actor%20Object%20Reference))
  ;[1 1 1] Event Start
  (|CallParentFunction InteractingCharacter)
  (bind _returnvalue (Actor|GetActorOfClass "/Game/ThirdPerson/Blueprints/BP_ThirdPerson_NPC.BP_ThirdPerson_NPC_C"))
  (Default|TimerrKey _returnvalue (Math|Random|RandomFloatinRange 0.2 0.3))
  (bind _ascharacter (Utilities|Casting|CastToCharacter (Variables|Default|GetInteractingActor)))
  (bind _output_get (Variables|Default|SetCharacter _ascharacter))
  (Class|BPICharacter|ToggleMovement(Message) _output_get false)
  (Animation|PlayAnimMontage _output_get "/Game/Characters/Mannequins/Animations/Manny/AI_Actions/Male_Sitting_Pose_Montage.Male_Sitting_Pose_Montage" 1.0 "None")
  (bind _returnvalue_2 (Actor|GetActorOfClass "/Game/GrabSystem/Demo/ThirdPersonBP/Blueprints/BP_ThirdPersonCharacter.BP_ThirdPersonCharacter_C"))
  (Default|Locatecostumer _returnvalue_2 (Transformation|GetActorLocation))
  (Components|MoveComponentTo (Variables|/Script/Engine.Actor|GetRootComponent (Variables|Default|GetCharacter)) (+ (Transformation|GetActorLocation) (Math|Vector|MakeVector 0.0 0.0 54.0)) (Math|Rotator|MakeRotator 0.0 0.0 0.0) true true 0.6 false))

(event EventCostumerCome?
  (params (NewParam :type Boolean))
  ;[1 1 1] Costumer Come
)

(fn ConstructionScript
  (|CallParentFunction))

(fn EndInteraction
  (|CallParentFunction)
  (CallFunction|ReleaseChair)
  (return true))